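; PC_Math is a debug test Blueprint, apparently a player controller, that displays where a test object sits relative to the pawn.
; On BeginPlay it caches the BP_CubeTest actor.
; Each Tick prints whether that actor is in front, plus its normalized and degree angles from helper functions defined outside this file.
; Print duration comes from the timecode frame interval, so readouts last roughly one frame.
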(event EventBeginPlay
  (bind _returnvalue (Actor|GetActorOfClass "/MathFunctions/BP_CubeTest.BP_CubeTest_C"))
  (Variables|Default|SetObject _returnvalue))

(event EventTick
  (params (DeltaSeconds :type Float%20%28single-precision%29))
  (bind _returnvalue (Class|TimeManagementBlueprintLibrary|GetTimecodeFrameRate))
  (bind _object (Variables|Default|GetObject))
  (bind _returnvalue_2 (Class|TimeManagementBlueprintLibrary|ToInterval(FrameRate) _returnvalue))
  (bind (_normalized _degrees) (CallFunction|DegreesAngletoObjectfromPawn _object))
  (Development|PrintString (Utilities|String|Append "In Front: " (Utilities|String|ToString(Boolean) (CallFunction|IsObjectinFrontOfPawn _object))) true true "(R=0.000000,G=0.660000,B=1.000000,A=1.000000)" _returnvalue_2)
  (Development|PrintString (Utilities|String|Append "Normalized Angle: " (Utilities|String|ToString(Float) _normalized)) true true "(R=0.000000,G=0.660000,B=1.000000,A=1.000000)" _returnvalue_2)
  (Development|PrintString (Utilities|String|Append "Angle in Degrees: " (Utilities|String|ToString(Float) _degrees)) true true "(R=0.000000,G=0.660000,B=1.000000,A=1.000000)" _returnvalue_2))

(fn ConstructionScript)